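; BP_GaiaPlayerController is a player controller that seeds a test inventory and shows it on screen at startup.
; After a one-second delay on BeginPlay, it creates a test container owned by itself through GaiaInventorySubsystem.
; A sequence then fills the container with three test item instances and opens its window through GaiaUIManagerSubsystem.
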(event `self.ReceiveBeginPlay`
  (bind _returnvalue (subsystem `GaiaInventorySubsystem`))
  (bind _returnvalue_2 (subsystem `GaiaInventorySubsystem`))
  (`KismetSystemLibrary.Delay` 1.0)
  (bind _returnvalue_3 (`GaiaInventorySubsystem.CreateContainerForPlayer` _returnvalue_2 "TestContainer" self))
  (`|ExecutionSequence`
    (:`then_0`
      (bind _returnvalue_4 (`GaiaInventorySubsystem.CreateItemInstance` _returnvalue_2 "TestItem" 1))
      (`GaiaInventorySubsystem.AddItemToContainer` _returnvalue_2 _returnvalue_4 _returnvalue_3)
      (bind _returnvalue_5 (`GaiaInventorySubsystem.CreateItemInstance` _returnvalue "TestItem2" 10))
      (`GaiaInventorySubsystem.AddItemToContainer` _returnvalue _returnvalue_5 _returnvalue_3)
      (bind _returnvalue_6 (`GaiaInventorySubsystem.CreateItemInstance` _returnvalue "TestItem3" 10))
      (`GaiaInventorySubsystem.AddItemToContainer` _returnvalue _returnvalue_6 _returnvalue_3))
    (:`then_1`
      (`GaiaUIManagerSubsystem.OpenContainerWindow` (subsystem `GaiaUIManagerSubsystem`) _returnvalue_3 false))))

(fn `UserConstructionScript`)